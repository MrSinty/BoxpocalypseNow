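; Megaphone actor that delivers tutorial and per-day start, random and end dialogue, and starts ambient and music audio on BeginPlay.
; It sorts DT_Dialogues rows into arrays by text type, which Speak selects from.
; SetSentence steps sequentially through lines in a WBP_Dialogue widget, with "random" sets gated by WillDisplay, then restores input and notifies the player character when finished.
; A timeline tilts the megaphone as it speaks.
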(event Custom|NextText
  (CallFunction|Speak (Variables|Default|GetTextType) (Variables|Default|GetWillDisplay?)))

(event Custom|PlayAnim
  (bind _speak (Timeline|SpeechAnim PlayFromStart)
    (:Update
      (Transformation|SetActorRotation (Math|Rotator|Lerp(Rotator) (Math|Rotator|MakeRotator 0.0 45.0 -9e+01) (Math|Rotator|MakeRotator 0.0 55.0 -9e+01) _speak)))))

(event EventSpeak
  (params (TextType :type E_TextTypes%20Enum :default "NewEnumerator4") (WillDisplayRandom? :type Boolean))
  (Variables|Default|SetWillDisplay? WillDisplayRandom?)
  (if (Utilities|Enum|NotEqual(Enum) TextType (Variables|Default|GetTextType))
    (Variables|Default|SetTextType TextType)
    (Variables|Default|SetFinishedBranch false))
  (if (Variables|Default|GetFinishedBranch)
    (Class|BPIDialogue|StopSpeak(Message) (Game|GetPlayerCharacter 0))
    (else
      (switch Utilities|FlowControl|Switch|SwitchonE_TextTypes (Variables|Default|GetTextType)
        (:NewEnumerator0
          (CallFunction|SetSentence (Variables|Default|GetTutorial) false))
        (:NewEnumerator1
          (CallFunction|SetSentence (Variables|Default|GetDay1Start) false))
        (:NewEnumerator2
          (CallFunction|SetSentence (Variables|Default|GetDay2Start) false))
        (:NewEnumerator3
          (CallFunction|SetSentence (Variables|Default|GetDay3Start) false))
        (:NewEnumerator5
          (CallFunction|SetSentence (Variables|Default|GetDay1Random) true))
        (:NewEnumerator6
          (CallFunction|SetSentence (Variables|Default|GetDay2Random) true))
        (:NewEnumerator7
          (CallFunction|SetSentence (Variables|Default|GetDay3Random) true))
        (:NewEnumerator8
          (CallFunction|SetSentence (Variables|Default|GetDay1End) false))
        (:NewEnumerator9
          (CallFunction|SetSentence (Variables|Default|GetDay2End) false))
        (:NewEnumerator10
          (CallFunction|SetSentence (Variables|Default|GetDay3End) false)))
      (CallFunction|PlayAnim))))

(event EventBeginPlay
  (CallFunction|LoadDialogues)
  (Audio|Components|Audio|Play (Variables|Default|GetSC_Ambient) 0.0)
  (Audio|Components|Audio|Play (Variables|Default|GetSC_RandomMusic) 0.0))

(fn ConstructionScript)

(fn SetSentence
  (params (TextToSet :type Array%20of%20Texts) (IsRandom :type Boolean))
  (LocalVariables|SetFullTextToSet TextToSet)
  (bind _output_get (LocalVariables|SetLIsRandom IsRandom))
  (if _output_get
    (if (Variables|Default|GetWillDisplay?)
      (Math|Integer|IncrementInt (Variables|Default|GettalkIndex) :!label _label
        (:%20%20
          (if (< (Variables|Default|GettalkIndex) (Utilities|Array|Length (LocalVariables|GetFullTextToSet)))
            (Variables|Default|GetUI_Text
              (:then
                _)
              (:else
                (bind _returnvalue (UserInterface|CreateWidget "/Game/Assets/Blueprints/Widgets/WBP_Dialogue.WBP_Dialogue_C" (Game|GetPlayerController 0)))
                (bind _output_get_2 (Variables|Default|SetUI_Text _returnvalue))
                (UserInterface|Viewport|AddtoViewport _output_get_2 0)
                (Input|SetInputModeUIOnly (Game|GetPlayerController 0) _output_get_2 "DoNotLock" false)))
            (if (LocalVariables|GetLIsRandom)
              (Utilities|FlowControl|DoOnce false
                (:Completed
                  _)))
            (Variables|/Game/Assets/Blueprints/Widgets/WBP_Dialogue.WBP_Dialogue_C|SetfullText (Variables|Default|GetUI_Text) (Utilities|Text|FormatText (Utilities|Array|Get(acopy) (LocalVariables|GetFullTextToSet) (Variables|Default|GettalkIndex)) (Utilities|Text|MakeLiteralText " ")))
            (Default|StartTextAnim (Variables|Default|GetUI_Text))
            (else
              (Variables|Default|SettalkIndex -1)
              (Variables|Default|SetFinishedBranch true)
              (Input|SetInputModeGameandUI (Game|GetPlayerController 0) 0 "LockOnCapture" false false)
              (Variables|Default|GetUI_Text
                (:then
                  (Widget|RemovefromParent (Variables|Default|GetUI_Text))
                  (Variables|Default|SetUI_Text 0))
                (:else
                  _))
              (Class|BPIDialogue|StopSpeak(Message) (Game|GetPlayerCharacter 0))))))
      (else
        (Class|BPIDialogue|StopSpeak(Message) (Game|GetPlayerCharacter 0))))
    (else
      (goto _label))))

(fn LoadDialogues
  (bind _outrownames (DataTable|GetDataTableRowNames "/Game/Assets/DataTables/DT_Dialogues.DT_Dialogues"))
  (for _array_element _outrownames
    (bind _returnvalue (Utilities|GetDataTableRow "/Game/Assets/DataTables/DT_Dialogues.DT_Dialogues" _array_element)
      (:then
        (switch Utilities|FlowControl|Switch|SwitchonE_TextTypes (.texttype _returnvalue)
          (:NewEnumerator0
            (Utilities|Array|Add (Variables|Default|GetTutorial) (.texttosay _returnvalue)))
          (:NewEnumerator1
            (Utilities|Array|Add (Variables|Default|GetDay1Start) (.texttosay _returnvalue)))
          (:NewEnumerator2
            (Utilities|Array|Add (Variables|Default|GetDay2Start) (.texttosay _returnvalue)))
          (:NewEnumerator3
            (Utilities|Array|Add (Variables|Default|GetDay3Start) (.texttosay _returnvalue)))
          (:NewEnumerator5
            (Utilities|Array|Add (Variables|Default|GetDay1Random) (.texttosay _returnvalue)))
          (:NewEnumerator6
            (Utilities|Array|Add (Variables|Default|GetDay2Random) (.texttosay _returnvalue)))
          (:NewEnumerator7
            (Utilities|Array|Add (Variables|Default|GetDay3Random) (.texttosay _returnvalue)))
          (:NewEnumerator8
            (Utilities|Array|Add (Variables|Default|GetDay1End) (.texttosay _returnvalue)))
          (:NewEnumerator9
            (Utilities|Array|Add (Variables|Default|GetDay2End) (.texttosay _returnvalue)))
          (:NewEnumerator10
            (Utilities|Array|Add (Variables|Default|GetDay3End) (.texttosay _returnvalue))))))))