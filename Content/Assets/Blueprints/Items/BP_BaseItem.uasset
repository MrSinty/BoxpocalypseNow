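; Base inspectable box item that generates as correct or faulty and responds to clicks.
; InitiateItem randomizes defect sprites and content mesh from DataTables, plus a rule-based sticker code.
; Faulty items randomize which parts fail, forcing a wrong sticker if box and content are both correct.
; Box clicks notify the spawner's character, while cap clicks toggle a Timeline flap animation and report the first opening to the spawner.
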(event OnClicked(CapCollider)
  (params (TouchedComponent :type Primitive%20Component%20Object%20Reference) (ButtonPressed :type Key%20Structure :default "None"))
  (if (and (== ButtonPressed "LeftMouseButton") (not (Variables|Default|GetnotClickable)))
    (Utilities|FlowControl|Sequence
      (:then_0
        ;[1 1 1] Notify char about cap opened and change bool states
        (Variables|Default|SethasClicked true)
        (Variables|Default|SetisOpened (not (Variables|Default|GetisOpened)))
        (if (not (Variables|Default|GetnowOpened))
          (Default|CapOpened (Variables|Default|GetItemSpawner))
          (Variables|Default|SetnowOpened true)))
      (:then_1
        ;[1 1 1] Cap Open Animation
        (Utilities|FlowControl|FlipFlop
          (:A
            (bind (_direction _rotatecap) (Timeline|Timeline Play)
              (:Update
                (switch Utilities|FlowControl|Switch|SwitchonETimelineDirection _direction
                  (:Forward
                    (Transformation|SetRelativeRotation (Variables|Default|GetBoxCap2) (Math|Rotator|MakeRotator _rotatecap 0.0 1.8e+02) false false)
                    (Transformation|SetRelativeRotation (Variables|Default|GetBoxCap1) (Math|Rotator|MakeRotator _rotatecap 0.0 0.0) false false))
                  (:Backward
                    (Transformation|SetRelativeRotation (Variables|Default|GetBoxCap2) (Math|Rotator|MakeRotator _rotatecap 0.0 1.8e+02) false false)
                    (Transformation|SetRelativeRotation (Variables|Default|GetBoxCap1) (Math|Rotator|MakeRotator _rotatecap 0.0 0.0) false false))))))
          (:B
            (Timeline|Timeline Reverse)))))))

(event OnClicked(BoxSMesh)
  (params (TouchedComponent :type Primitive%20Component%20Object%20Reference) (ButtonPressed :type Key%20Structure :default "None"))
  (if (and (== ButtonPressed "LeftMouseButton") (not (Variables|Default|GetnotClickable)))
    (Default|ItemPressed (Variables|/Game/Assets/Blueprints/Items/BP_ItemSpawner.BP_ItemSpawner_C|GetCharBP (Variables|Default|GetItemSpawner)))))

(fn ConstructionScript)

(fn RandomSticker
  (params (IsCorrectSticker :type Boolean)))

(fn RandomBoxContent
  (params (IsBoxContentCorrect :type Boolean))
  (bind _outrownames (DataTable|GetDataTableRowNames "/Game/Assets/DataTables/DT_BoxContent.DT_BoxContent"))
  (LocalVariables|SetRowNames _outrownames)
  (bind _returnvalue (Utilities|GetDataTableRow "/Game/Assets/DataTables/DT_BoxContent.DT_BoxContent" (.OutItem (Utilities|Array|Random (LocalVariables|GetRowNames))))
    (:then
      (LocalVariables|SetRandomMesh (.staticmesh _returnvalue))
      (LocalVariables|SetIsRandomCorrect (.iscorrect _returnvalue))
      (while (!= IsBoxContentCorrect (LocalVariables|GetIsRandomCorrect))
        (bind _returnvalue_2 (Utilities|GetDataTableRow "/Game/Assets/DataTables/DT_BoxContent.DT_BoxContent" (.OutItem (Utilities|Array|Random (LocalVariables|GetRowNames))))
          (:then
            (LocalVariables|SetRandomMesh (.staticmesh _returnvalue_2))
            (LocalVariables|SetIsRandomCorrect (.iscorrect _returnvalue_2)))))
      (Components|StaticMesh|SetStaticMesh (Variables|Default|GetBoxContentMesh) (LocalVariables|GetRandomMesh)))))

(fn AdjustBoxLocation
  (bind _returnvalue (Math|Float|MakeLiteralFloat 2.0))
  (bind _boxsmesh (Variables|Default|GetBoxSMesh))
  (bind _boxextent (Collision|GetComponentBounds _boxsmesh))
  (bind _returnvalue_2 (/ _boxextent _returnvalue))
  (bind _z (Math|Vector|BreakVector _returnvalue_2))
  (Transformation|SetRelativeLocation (Variables|Default|GetArrow) (Math|Vector|MakeVector 0.0 0.0 _z) false false)
  (Transformation|SetRelativeLocation (Variables|Default|GetBoxSMesh) (* (Math|Vector|MakeVector 0.0 0.0 _z) (Math|Float|MakeLiteralFloat -1.0)) false false))

(fn RandomBoxDefects
  (params (IsBoxCorrect :type Boolean))
  (if IsBoxCorrect
    (return)
    (else
      (bind _outrownames (DataTable|GetDataTableRowNames "/Game/Assets/Materials/BoxBrokenness/DT_Defects.DT_Defects"))
      (LocalVariables|SetDT_Rows _outrownames)
      (for _index (range 0 (Math|Random|RandomIntegerinRange 0 2))
        (bind _returnvalue (Utilities|GetDataTableRow "/Game/Assets/Materials/BoxBrokenness/DT_Defects.DT_Defects" (.OutItem (Utilities|Array|Random (LocalVariables|GetDT_Rows))))
          (:then
            (Utilities|Array|Add (Variables|Default|GetRandDefectSprites) (.sprite _returnvalue))))))))

(fn InitiateItem
  (params (IsCorrect :type Boolean))
  (bind _output_get (Variables|Default|SetisUnbroken IsCorrect))
  (if _output_get
    (CallFunction|RandomBoxDefects true)
    (CallFunction|AdjustBoxLocation)
    (CallFunction|RandomBoxContent true)
    (CallFunction|SetStickerText true)
    (CallFunction|AssignDefects)
    (else
      (bind _output_get_2 (LocalVariables|SetBox (Math|Random|RandomBool)))
      (CallFunction|RandomBoxDefects _output_get_2)
      (CallFunction|AdjustBoxLocation)
      (bind _output_get_3 (LocalVariables|SetBoxContent (Math|Random|RandomBool)))
      (CallFunction|RandomBoxContent _output_get_3)
      (if (and (LocalVariables|GetBox) (LocalVariables|GetBoxContent))
        (CallFunction|SetStickerText false)
        (else
          (CallFunction|SetStickerText (Math|Random|RandomBool))))
      (CallFunction|AssignDefects))))

(fn SetStickerText
  (params (IsStikerCorrect :type Boolean))
  (if IsStikerCorrect
    (for _index (range 0 5)
      (if (== _index 1)
        (CallFunction|AddRandomChar (LocalVariables|GetCharsCapital) (LocalVariables|GetStickerText))
        (elif (== _index 4)
          (CallFunction|AddRandomChar (LocalVariables|GetVowels) (LocalVariables|GetStickerText))
          (else
            (CallFunction|AddRandomChar (LocalVariables|GetAllSymbols) (LocalVariables|GetStickerText))))))
    (CallFunction|AddRandomChar (LocalVariables|GetEvenNums) (LocalVariables|GetStickerText))
    (Rendering|Components|TextRender|SetText (Variables|Default|GetSticker_text) (Utilities|Text|ToText(String) (LocalVariables|GetStickerText)))
    (else
      (LocalVariables|SetCapital (Math|Random|RandomBool))
      (LocalVariables|SetVowel (Math|Random|RandomBool))
      (if (or (LocalVariables|GetCapital) (LocalVariables|GetVowel))
        (LocalVariables|SetEven (Math|Random|RandomBool))
        (else
          (LocalVariables|SetEven true)))
      (Utilities|FlowControl|Sequence
        (:then_0
          (if (LocalVariables|GetVowel)
            (for _array_element (Utilities|String|GetCharacterArrayfromString (LocalVariables|GetVowels))
              (|SetBy-RefVar (LocalVariables|GetWrongSymbols) (Utilities|String|Replace (LocalVariables|GetWrongSymbols) _array_element)))))
        (:then_1
          (if (LocalVariables|GetCapital)
            (for _array_element_2 (Utilities|String|GetCharacterArrayfromString (LocalVariables|GetCharsCapital))
              (|SetBy-RefVar (LocalVariables|GetWrongSymbols) (Utilities|String|Replace (LocalVariables|GetWrongSymbols) _array_element_2 "" "CaseSensitive")))))
        (:then_2
          (for _index_2 (range 0 5)
            (CallFunction|AddRandomChar (LocalVariables|GetWrongSymbols) (LocalVariables|GetStickerText)))
          (if (LocalVariables|GetEven)
            (CallFunction|AddRandomChar (LocalVariables|GetOddNums) (LocalVariables|GetStickerText))
            (else
              (CallFunction|AddRandomChar (LocalVariables|GetEvenNums) (LocalVariables|GetStickerText))))
          (Rendering|Components|TextRender|SetText (Variables|Default|GetSticker_text) (Utilities|Text|ToText(String) (LocalVariables|GetStickerText))))))))

(fn AssignDefects
  (bind _randdefectsprites (Variables|Default|GetRandDefectSprites))
  (bind _defectcomps (LocalVariables|GetDefectComps))
  (bind _returnvalue (Utilities|Array|Length _randdefectsprites))
  (Utilities|Array|Add _defectcomps (Variables|Default|GetDefect1))
  (Utilities|Array|Add _defectcomps (Variables|Default|GetDefect2))
  (Utilities|Array|Add _defectcomps (Variables|Default|GetDefect3))
  (if (!= _returnvalue 0)
    (bind _index (Utilities|FlowControl|ForLoopwithBreak 0 (- _returnvalue 1))
      (:LoopBody
        (Rendering|Components|Sprite|SetSprite (Utilities|Array|Get(acopy) (LocalVariables|GetDefectComps) _index) (Utilities|Array|Get(acopy) _randdefectsprites _index))
        (Transformation|SetRelativeScale3D (Utilities|Array|Get(acopy) (LocalVariables|GetDefectComps) _index) "0.020000,0.020000,0.020000")))))

(fn AddRandomChar
  (params (Add%20from :type String%20%28by%20ref%29) (Add%20to :type String%20%28by%20ref%29))
  (|SetBy-RefVar Add%20to (Utilities|String|Append Add%20to (.OutItem (Utilities|Array|Random (Utilities|String|GetCharacterArrayfromString Add%20from))))))