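; BP_Button_Correct is a clickable button actor that represents the correct choice.
; Clicking it calls PressedCorrectMessage on player character 0, plays the SCButton component and restarts the ButtonAnim timeline, which drives the Button component's relative location.
; The construction script applies a fixed material, named with a green hex color, to the Button.
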(event EventBeginPlay
  (|CallParentFunction) ; This node is disabled and will not be called.\nDrag off pins to build functionality.
)

(event Collision|EventActorBeginOverlap
  (params (OtherActor :type Actor%20Object%20Reference))
  (|CallParentFunction OtherActor) ; This node is disabled and will not be called.\nDrag off pins to build functionality.
)

(event EventTick
  (params (DeltaSeconds :type Float%20%28single-precision%29))
  (|CallParentFunction DeltaSeconds) ; This node is disabled and will not be called.\nDrag off pins to build functionality.
)

(event MouseInput|EventActorOnClicked
  (params (ButtonPressed :type Key%20Structure :default "None"))
  (Class|BPIButtons|PressedCorrect(Message) (Game|GetPlayerCharacter 0))
  (Audio|Components|Audio|Play (Variables|Default|GetSC_Button) 0.0)
  (bind _changelocation (Timeline|ButtonAnim PlayFromStart)
    (:Update
      (Transformation|SetRelativeLocation (Variables|Default|GetButton) _changelocation false false))))

(fn ConstructionScript
  (|CallParentFunction)
  (Rendering|Material|SetMaterial (Variables|Default|GetButton) 0 "/Game/Assets/Meshes/Buttons/46F500FF.46F500FF"))