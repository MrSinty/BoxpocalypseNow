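; BP_ItemSpawnerMenu runs an endless conveyor display of items, apparently for the menu.
; It spawns the output item of a random entry in BoxesBPs at its own location and initiates it.
; Two chained timelines linearly move the item to a work point, then to an end point, playing the conveyor sound or component at each leg.
; The item is then destroyed and the next one spawns.
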(event Custom|SpawnNewItem
  (bind _returnvalue (Game|SpawnActorfromClass (.OutItem (Utilities|Array|Random (Variables|Default|GetBoxesBPs))) (Transformation|GetWorldTransform (Variables|Default|GetDefaultSceneRoot)) "AlwaysSpawn" "MultiplyWithRoot" 0 0))
  (Variables|Default|SetItemOnScene _returnvalue)
  (Default|InitiateItem (Variables|Default|GetItemOnScene))
  (CallFunction|MovetoWork))

(event Custom|MoveToWork
  (Audio|Components|Audio|Play (Variables|Default|GetSC_Conveyour) 0.0)
  (bind _fromstarttowork (Timeline|StartToWork PlayFromStart)
    (:Update
      (CallFunction|MovetoPosition (Variables|Default|GetItemOnScene) (Variables|Default|GetStartPoint) (Variables|Default|GetWorkPoint) _fromstarttowork))
    (:Finished
      (CallFunction|MovetoEnd))))

(event Custom|MoveToEnd
  (Audio|Components|Audio|Play (Variables|Default|GetSC_Conveyour) 0.0)
  (bind _fromworktoend (Timeline|WorkToEnd PlayFromStart)
    (:Update
      (CallFunction|MovetoPosition (Variables|Default|GetItemOnScene) (Variables|Default|GetWorkPoint) (Variables|Default|GetEndPoint) _fromworktoend))
    (:Finished
      (Actor|DestroyActor (Variables|Default|GetItemOnScene))
      (CallFunction|SpawnNewItem))))

(event EventBeginPlay
  (Variables|Default|SetStartPoint (Transformation|GetWorldLocation (Variables|Default|GetDefaultSceneRoot)))
  (CallFunction|SpawnNewItem))

(fn ConstructionScript)

(fn MovetoPosition
  (params (ItemToMove :type BP%20Base%20Item%20Menu%20Object%20Reference) (Start :type Vector) (End :type Vector) (TimeLineFloat :type Float%20%28double-precision%29))
  (Transformation|SetWorldLocation (Variables|/Script/Engine.Actor|GetRootComponent ItemToMove) (+ Start (* (- End Start) TimeLineFloat)) false false))