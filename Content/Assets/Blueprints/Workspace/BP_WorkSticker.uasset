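; BP_WorkSticker is a workspace sticker that displays a box counter as "current/total" text.
; SetAmountOfBoxes and SetNumberOfBox store the total and current values passed in by callers, then each calls ChangeText.
; ChangeText joins both numbers with a slash and writes the result to the NumOfBoxes text element.
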(event Custom|ChangeText
  (Rendering|Components|TextRender|SetText (Variables|Default|GetNumOfBoxes) (Utilities|Text|ToText(String) (Utilities|String|Append (Utilities|String|ToString(Integer) (Variables|Default|GetNumOfBox)) "/" (Utilities|String|ToString(Integer) (Variables|Default|GetAmountOfBoxes))))))

(event EventSetNumberOfBox
  (params (NumOfBox :type Integer))
  (Variables|Default|SetNumOfBox NumOfBox)
  (CallFunction|ChangeText))

(event EventSetAmountOfBoxes
  (params (AmountBoxes :type Integer))
  (Variables|Default|SetAmountOfBoxes AmountBoxes)
  (CallFunction|ChangeText))

(fn ConstructionScript)