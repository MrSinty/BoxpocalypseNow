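; Base menu item: a box that randomizes its sticker code and surface defects, each independently correct or faulty.
; InitiateItem adds up to three DT_Defects sprites, offsets box and arrow by mesh bounds, builds sticker text and applies sprites.
; Valid codes place a capital and vowel at fixed positions and end in an even digit; faulty ones strip characters from the pool or end odd.
; RandomSticker's numeric labeling is disconnected.
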(fn ConstructionScript)

(fn RandomSticker
  (params (IsCorrectSticker :type Boolean)))

(fn AdjustBoxLocation
  (bind _returnvalue (Math|Float|MakeLiteralFloat 2.0))
  (bind _boxmesh (Variables|Default|GetBoxMesh))
  (bind _boxextent (Collision|GetComponentBounds _boxmesh))
  (bind _returnvalue_2 (/ _boxextent _returnvalue))
  (bind _z (Math|Vector|BreakVector _returnvalue_2))
  (Transformation|SetRelativeLocation (Variables|Default|GetArrow) (Math|Vector|MakeVector 0.0 0.0 _z) false false)
  (Transformation|SetRelativeLocation (Variables|Default|GetBoxMesh) (* (Math|Vector|MakeVector 0.0 0.0 _z) (Math|Float|MakeLiteralFloat -1.0)) false false))

(fn RandomBoxDefects
  (params (IsBoxCorrect :type Boolean))
  (if IsBoxCorrect
    (return)
    (else
      (bind _outrownames (DataTable|GetDataTableRowNames "/Game/Assets/Materials/BoxBrokenness/DT_Defects.DT_Defects"))
      (LocalVariables|SetDT_Rows _outrownames)
      (for _index (range 0 (Math|Random|RandomIntegerinRange 0 2))
        (bind _returnvalue (Utilities|GetDataTableRow "/Game/Assets/Materials/BoxBrokenness/DT_Defects.DT_Defects" (.OutItem (Utilities|Array|Random (LocalVariables|GetDT_Rows))))
          (:then
            (Utilities|Array|Add (Variables|Default|GetRandDefectSprites) (.sprite _returnvalue))))))))

(fn InitiateItem
  (CallFunction|RandomBoxDefects (Math|Random|RandomBool))
  (CallFunction|AdjustBoxLocation)
  (CallFunction|SetStickerText (Math|Random|RandomBool))
  (CallFunction|AssignDefects))

(fn SetStickerText
  (params (IsStikerCorrect :type Boolean))
  (if IsStikerCorrect
    (for _index (range 0 5)
      (if (== _index 1)
        (CallFunction|AddRandomChar (LocalVariables|GetCharsCapital) (LocalVariables|GetStickerText))
        (elif (== _index 4)
          (CallFunction|AddRandomChar (LocalVariables|GetVowels) (LocalVariables|GetStickerText))
          (else
            (CallFunction|AddRandomChar (LocalVariables|GetAllSymbols) (LocalVariables|GetStickerText))))))
    (CallFunction|AddRandomChar (LocalVariables|GetEvenNums) (LocalVariables|GetStickerText))
    (Rendering|Components|TextRender|SetText (Variables|Default|GetSticker_text) (Utilities|Text|ToText(String) (LocalVariables|GetStickerText)))
    (else
      (LocalVariables|SetCapital (Math|Random|RandomBool))
      (LocalVariables|SetVowel (Math|Random|RandomBool))
      (if (or (LocalVariables|GetCapital) (LocalVariables|GetVowel))
        (LocalVariables|SetEven (Math|Random|RandomBool))
        (else
          (LocalVariables|SetEven true)))
      (Utilities|FlowControl|Sequence
        (:then_0
          (if (LocalVariables|GetVowel)
            (for _array_element (Utilities|String|GetCharacterArrayfromString (LocalVariables|GetVowels))
              (|SetBy-RefVar (LocalVariables|GetWrongSymbols) (Utilities|String|Replace (LocalVariables|GetWrongSymbols) _array_element)))))
        (:then_1
          (if (LocalVariables|GetCapital)
            (for _array_element_2 (Utilities|String|GetCharacterArrayfromString (LocalVariables|GetCharsCapital))
              (|SetBy-RefVar (LocalVariables|GetWrongSymbols) (Utilities|String|Replace (LocalVariables|GetWrongSymbols) _array_element_2 "" "CaseSensitive")))))
        (:then_2
          (for _index_2 (range 0 5)
            (CallFunction|AddRandomChar (LocalVariables|GetWrongSymbols) (LocalVariables|GetStickerText)))
          (if (LocalVariables|GetEven)
            (CallFunction|AddRandomChar (LocalVariables|GetOddNums) (LocalVariables|GetStickerText))
            (else
              (CallFunction|AddRandomChar (LocalVariables|GetEvenNums) (LocalVariables|GetStickerText))))
          (Rendering|Components|TextRender|SetText (Variables|Default|GetSticker_text) (Utilities|Text|ToText(String) (LocalVariables|GetStickerText))))))))

(fn AssignDefects
  (bind _randdefectsprites (Variables|Default|GetRandDefectSprites))
  (bind _defectcomps (LocalVariables|GetDefectComps))
  (bind _returnvalue (Utilities|Array|Length _randdefectsprites))
  (Utilities|Array|Add _defectcomps (Variables|Default|GetDefect1))
  (Utilities|Array|Add _defectcomps (Variables|Default|GetDefect2))
  (Utilities|Array|Add _defectcomps (Variables|Default|GetDefect3))
  (if (!= _returnvalue 0)
    (bind _index (Utilities|FlowControl|ForLoopwithBreak 0 (- _returnvalue 1))
      (:LoopBody
        (Rendering|Components|Sprite|SetSprite (Utilities|Array|Get(acopy) (LocalVariables|GetDefectComps) _index) (Utilities|Array|Get(acopy) _randdefectsprites _index))
        (Transformation|SetRelativeScale3D (Utilities|Array|Get(acopy) (LocalVariables|GetDefectComps) _index) "0.020000,0.020000,0.020000")))))

(fn AddRandomChar
  (params (Add%20from :type String%20%28by%20ref%29) (Add%20to :type String%20%28by%20ref%29))
  (|SetBy-RefVar Add%20to (Utilities|String|Append Add%20to (.OutItem (Utilities|Array|Random (Utilities|String|GetCharacterArrayfromString Add%20from))))))