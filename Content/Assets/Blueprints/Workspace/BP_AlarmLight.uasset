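; BP_AlarmLight is an alarm light that signals an error with a rotating red spotlight and a sound.
; Its ErrorLighton event unhides the SpotLight, tints it red, plays WrongAudio from a start offset and restarts the RotateLight timeline.
; Each timeline update adds the track value as a local pitch rotation, and the light is hidden again when the timeline finishes.
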(event EventErrorLighton
  (Development|SetHiddeninGame (Variables|Default|GetSpotLight) false false)
  (Rendering|Components|Light|SetLightColor (Variables|Default|GetSpotLight) (Math|Color|MakeColor 1.0 0.0 0.0) true)
  (Audio|Components|Audio|Play (Variables|Default|GetWrongAudio) 0.5)
  (bind _rotatelight (Timeline|RotateLight PlayFromStart)
    (:Update
      (Transformation|AddLocalRotation (Variables|Default|GetSpotLight) (Math|Rotator|MakeRotator 0.0 _rotatelight 0.0) false false))
    (:Finished
      (Development|SetHiddeninGame (Variables|Default|GetSpotLight) true false))))

(fn ConstructionScript)