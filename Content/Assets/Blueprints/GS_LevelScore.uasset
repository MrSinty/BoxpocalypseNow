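; Level score state that tracks the player's item-judging score and end-of-day food and beer choices.
; Correct and Wrong button handlers check the ItemSpawner's broken-item flag to raise or lower Score.
; SaveDayChoices archives each day's three choices into EndDaysLog, then clears them.
; CheckGameOver tallies logged days without food or beer and shows the game-over widget when either count reaches its limit.
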(event Custom|SaveDayChoices
  (Utilities|Array|Add (Variables|Default|GetEndDaysLog) (Utilities|Struct|MakeS_EndDaysLog (Utilities|Array|Get(acopy) (Variables|Default|GetEndDayChoices)) (Utilities|Array|Get(acopy) (Variables|Default|GetEndDayChoices) 1) (Utilities|Array|Get(acopy) (Variables|Default|GetEndDayChoices) 2)))
  (Utilities|Array|Clear (Variables|Default|GetEndDayChoices)))

(event Custom|CheckGameOver
  (for _array_element (Variables|Default|GetEndDaysLog)
    (Utilities|FlowControl|Sequence
      (:then_0
        (if (not (.food _array_element))
          (Math|Integer|IncrementInt (Variables|Default|GetNoFoodCount))))
      (:then_1
        (if (not (.beer _array_element))
          (Math|Integer|IncrementInt (Variables|Default|GetNoBeerCount))))))
  (if (or (>= (Variables|Default|GetNoFoodCount) 2) (>= (Variables|Default|GetNoBeerCount) 3))
    (bind _returnvalue (UserInterface|CreateWidget "/Game/Assets/Blueprints/Widgets/WBP_GameOver.WBP_GameOver_C"))
    (UserInterface|Viewport|AddtoViewport _returnvalue 1)))

(fn ConstructionScript)

(fn CorrectBtnPressed
  (bind _isunbroken (Default|IsItemBroken (Utilities|ResolveSoftReference (Variables|Default|GetItemSpawner))))
  (if _isunbroken
    (Variables|Default|SetScore (+ (Variables|Default|GetScore) 4))
    (else
      (Variables|Default|SetScore (- (Variables|Default|GetScore) 3)))))

(fn WrongBtnPressed
  (bind _isunbroken (Default|IsItemBroken (Utilities|ResolveSoftReference (Variables|Default|GetItemSpawner))))
  (if _isunbroken
    (Variables|Default|SetScore (- (Variables|Default|GetScore) 3))
    (else
      (Variables|Default|SetScore (+ (Variables|Default|GetScore) 4)))))