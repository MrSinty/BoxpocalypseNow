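; BP_Exit is an exit door that lets the player finish the day once it has ended.
; On BeginPlay it finds and caches the BP_ItemSpawner, which holds the end-of-day and door-clicked flags.
; DoorClicked checks those flags, then calls EndDayWidget on the spawner's character reference, marks the door clicked to block repeats, and plays the door-opened sound.
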(event Custom|DoorClicked
  (bind _itemspawner (Variables|Default|GetItemSpawner))
  (if (and (not (Variables|/Game/Assets/Blueprints/Items/BP_ItemSpawner.BP_ItemSpawner_C|GetisClickedDoor _itemspawner)) (Variables|/Game/Assets/Blueprints/Items/BP_ItemSpawner.BP_ItemSpawner_C|GetisEndOfDay _itemspawner))
    (Default|EndDayWidget (Variables|/Game/Assets/Blueprints/Items/BP_ItemSpawner.BP_ItemSpawner_C|GetCharBP _itemspawner))
    (Variables|/Game/Assets/Blueprints/Items/BP_ItemSpawner.BP_ItemSpawner_C|SetisClickedDoor _itemspawner true)
    (Audio|Components|Audio|Play (Variables|Default|GetSC_DoorOpened) 0.0)))

(event EventBeginPlay
  (bind _returnvalue (Actor|GetActorOfClass "/Game/Assets/Blueprints/Items/BP_ItemSpawner.BP_ItemSpawner_C"))
  (Variables|Default|SetItemSpawner _returnvalue))

(fn ConstructionScript)