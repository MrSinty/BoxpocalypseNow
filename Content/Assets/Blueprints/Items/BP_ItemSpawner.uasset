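; Item spawner for a box-inspection job: feeds each day's queue of boxes along a conveyor to a work point for the player to examine.
; StartDay loads box types from per-day DataTables; SpawnItem spawns a random box class flagged intact, broken or random, updating the WorkSticker counter.
; Timelines lerp items to work and end points and toward the camera for rotatable inspection, blocking clicks while moving.
; An exhausted queue triggers end-of-day state and dialogue.
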(event Custom|SpawnNewItem
  (bind _returnvalue (Game|SpawnActorfromClass (.OutItem (Utilities|Array|Random (Variables|Default|GetBoxesBPs))) (Transformation|GetWorldTransform (Variables|Default|GetDefaultSceneRoot)) "AlwaysSpawn" "MultiplyWithRoot" 0 0))
  (bind _output_get (Variables|Default|SetItemOnScene _returnvalue))
  (Variables|/Game/Assets/Blueprints/Items/BP_BaseItem.BP_BaseItem_C|SetItemSpawner _output_get self)
  (Default|InitiateItem (Variables|Default|GetItemOnScene) (Math|Random|RandomBool))
  (CallFunction|MovetoWork))

(event Custom|MoveToWork
  (Variables|/Game/Assets/Blueprints/Items/BP_BaseItem.BP_BaseItem_C|SetnotClickable (Variables|Default|GetItemOnScene) true)
  (Audio|Components|Audio|Play (Variables|Default|GetSC_Conveyour) 0.0)
  (bind _fromstarttowork (Timeline|StartToWork PlayFromStart)
    (:Update
      (CallFunction|MovetoPosition (Variables|Default|GetItemOnScene) (Variables|Default|GetStartPoint) (Variables|Default|GetWorkPoint) _fromstarttowork))
    (:Finished
      (Variables|/Game/Assets/Blueprints/Items/BP_BaseItem.BP_BaseItem_C|SetnotClickable (Variables|Default|GetItemOnScene) false))))

(event Custom|MoveToEnd
  (Variables|/Game/Assets/Blueprints/Items/BP_BaseItem.BP_BaseItem_C|SetnotClickable (Variables|Default|GetItemOnScene) true)
  (Audio|Components|Audio|Play (Variables|Default|GetSC_Conveyour) 0.0)
  (bind _fromworktoend (Timeline|WorkToEnd PlayFromStart)
    (:Update
      (CallFunction|MovetoPosition (Variables|Default|GetItemOnScene) (Variables|Default|GetWorkPoint) (Variables|Default|GetEndPoint) _fromworktoend))
    (:Finished
      (Variables|/Game/Assets/Blueprints/Items/BP_BaseItem.BP_BaseItem_C|SetnotClickable (Variables|Default|GetItemOnScene) false)
      (Actor|DestroyActor (Variables|Default|GetItemOnScene))
      (CallFunction|SpawnItem))))

(event Custom|ClickedOnItem
  (Variables|/Game/Assets/Blueprints/Items/BP_BaseItem.BP_BaseItem_C|SetnotClickable (Variables|Default|GetItemOnScene) true)
  (Audio|Components|Audio|Play (Variables|Default|GetSC_TakeBox) 0.0)
  (bind (_direction _movetoplayercamera _changerotation) (Timeline|MoveTo/FromRotPoint Play)
    (:Update
      (CallFunction|MovetoScreen _movetoplayercamera _changerotation _direction))
    (:Finished
      (Variables|/Game/Assets/Blueprints/Items/BP_BaseItem.BP_BaseItem_C|SetnotClickable (Variables|Default|GetItemOnScene) false))))

(event Custom|UnclickedOnItem
  (Variables|/Game/Assets/Blueprints/Items/BP_BaseItem.BP_BaseItem_C|SetCurRotation (Variables|Default|GetItemOnScene) (Transformation|GetWorldRotation (Variables|/Game/Assets/Blueprints/Items/BP_BaseItem.BP_BaseItem_C|GetArrow (Variables|Default|GetItemOnScene))))
  (Variables|/Game/Assets/Blueprints/Items/BP_BaseItem.BP_BaseItem_C|SetnotClickable (Variables|Default|GetItemOnScene) true)
  (Audio|Components|Audio|Play (Variables|Default|GetSC_TakeBox) 0.0)
  (bind (_direction _movetoplayercamera _changerotation) (Timeline|MoveTo/FromRotPoint Reverse)
    (:Update
      (CallFunction|MovetoScreen _movetoplayercamera _changerotation _direction))
    (:Finished
      (Variables|/Game/Assets/Blueprints/Items/BP_BaseItem.BP_BaseItem_C|SetnotClickable (Variables|Default|GetItemOnScene) false))))

(event Custom|Start%20Day
  (CallFunction|LoadItemsforDay)
  (Variables|Default|SetIndexOfBoxType 0)
  (Variables|Default|SetisStartDay true)
  (Variables|Default|SetisEndOfDay false)
  (CallFunction|SpawnItem)
  (Default|RandomDialogue (Variables|Default|GetCharBP)))

(event Custom|EndOfDay
  (CallFunction|ChangeDayState)
  (Variables|Default|SetisClickedDoor false)
  (Default|EndDayDialogue (Variables|Default|GetCharBP)))

(event Custom|CapOpened
  (Default|CapOpened (Variables|Default|GetCharBP)))

(event EventBeginPlay
  (Variables|Default|SetStartPoint (Transformation|GetWorldLocation (Variables|Default|GetDefaultSceneRoot)))
  (bind _asbp_first_person_character (Utilities|Casting|CastToBP_FirstPersonCharacter (Game|GetPlayerCharacter 0)))
  (Variables|Default|SetCharBP _asbp_first_person_character))

(fn ConstructionScript)

(fn MovetoPosition
  (params (ItemToMove :type BP%20Base%20Item%20Object%20Reference) (Start :type Vector) (End :type Vector) (TimeLineFloat :type Float%20%28double-precision%29))
  (Transformation|SetWorldLocation (Variables|/Script/Engine.Actor|GetRootComponent ItemToMove) (+ Start (* (- End Start) TimeLineFloat)) false false))

(fn MovetofromCamera
  (params (NewLocation :type Vector) (NewRotation :type Rotator))
  (Transformation|SetWorldLocation (Variables|/Game/Assets/Blueprints/Items/BP_BaseItem.BP_BaseItem_C|GetDefaultSceneRoot (Variables|Default|GetItemOnScene)) NewLocation false false)
  (Transformation|SetWorldRotation (Variables|/Game/Assets/Blueprints/Items/BP_BaseItem.BP_BaseItem_C|GetArrow (Variables|Default|GetItemOnScene)) NewRotation false false))

(fn RotateItem
  (params (MouseX :type Float%20%28double-precision%29) (MouseY :type Float%20%28double-precision%29))
  (bind _returnvalue (Math|Float|MakeLiteralFloat -1e+01))
  (Transformation|AddWorldRotation (Variables|/Game/Assets/Blueprints/Items/BP_BaseItem.BP_BaseItem_C|GetArrow (Variables|Default|GetItemOnScene)) (Math|Rotator|MakeRotator (* MouseY _returnvalue) 0.0 (* MouseX _returnvalue)) false false))

(fn IsItemBroken
  (return (Variables|/Game/Assets/Blueprints/Items/BP_BaseItem.BP_BaseItem_C|GetisUnbroken (Variables|Default|GetItemOnScene))))

(fn MovetoScreen
  (params (TimelineMove :type Float%20%28double-precision%29) (TimelineRotation :type Float%20%28double-precision%29) (TimelineDirection :type ETimelineDirection%20Enum :default "Forward"))
  (bind _workpoint (Variables|Default|GetWorkPoint))
  (bind _rotationpoint (Variables|Default|GetRotationPoint))
  (bind _returnvalue (- _rotationpoint _workpoint))
  (bind _returnvalue_2 (* _returnvalue TimelineMove))
  (bind _returnvalue_3 (+ _workpoint _returnvalue_2))
  (switch Utilities|FlowControl|Switch|SwitchonETimelineDirection TimelineDirection
    (:Forward
      (CallFunction|MovetofromCamera _returnvalue_3 "0, 0, 0"))
    (:Backward
      (CallFunction|MovetofromCamera _returnvalue_3 (Math|Rotator|Lerp(Rotator) (Math|Rotator|MakeRotator 0.0 0.0 0.0) (Variables|/Game/Assets/Blueprints/Items/BP_BaseItem.BP_BaseItem_C|GetCurRotation (Variables|Default|GetItemOnScene)) TimelineRotation true)))))

(fn ChangeDayState
  (Utilities|FlowControl|FlipFlop
    (:A
      (Variables|Default|SetisStartDay false)
      (Variables|Default|SetisEndOfDay true))
    (:B
      (Variables|Default|SetisStartDay true)
      (Variables|Default|SetisEndOfDay false))))

(fn SpawnItem
  (bind _boxestypes (Variables|Default|GetBoxesTypes))
  (bind _indexofboxtype (Variables|Default|GetIndexOfBoxType))
  (Class|BPIAmountOfBoxes|SetNumberOfBox(Message) (Utilities|ResolveSoftReference (Variables|Default|GetWorkSticker)) (Variables|Default|GetIndexOfBoxType))
  (if (== _indexofboxtype (Utilities|Array|Length _boxestypes))
    (Variables|Default|SetisEndingDay true)
    (CallFunction|EndOfDay)
    (else
      (LocalVariables|SetBoxType (Utilities|Array|Get(acopy) _boxestypes _indexofboxtype))
      (Math|Integer|IncrementInt (Variables|Default|GetIndexOfBoxType)
        (:%20%20
          (bind _returnvalue (Game|SpawnActorfromClass (.OutItem (Utilities|Array|Random (Variables|Default|GetBoxesBPs))) (Transformation|GetWorldTransform (Variables|Default|GetDefaultSceneRoot)) "AlwaysSpawn" "MultiplyWithRoot" 0 0))
          (bind _output_get (Variables|Default|SetItemOnScene _returnvalue))
          (Variables|/Game/Assets/Blueprints/Items/BP_BaseItem.BP_BaseItem_C|SetItemSpawner _output_get self)
          (switch Utilities|FlowControl|Switch|SwitchonE_BoxTypes (LocalVariables|GetBoxType)
            (:NewEnumerator0
              (Default|InitiateItem (Variables|Default|GetItemOnScene) true))
            (:NewEnumerator1
              (Default|InitiateItem (Variables|Default|GetItemOnScene) false))
            (:NewEnumerator2
              (Default|InitiateItem (Variables|Default|GetItemOnScene) (Math|Random|RandomBool))))
          (CallFunction|MovetoWork))))))

(fn LoadItemsforDay
  (Utilities|Array|Clear (Variables|Default|GetBoxesTypes))
  (switch int (- (Variables|/Game/Assets/Blueprints/GS_LevelScore.GS_LevelScore_C|GetNumberOfDay (Variables|/Game/FirstPerson/Blueprints/BP_FirstPersonCharacter.BP_FirstPersonCharacter_C|GetGS%20Level%20Score (Variables|Default|GetCharBP))) 1)
    (:0
      (bind _outrownames (DataTable|GetDataTableRowNames "/Game/Assets/DataTables/DT_BoxTypesForDay1.DT_BoxTypesForDay1"))
      (Class|BPIAmountOfBoxes|SetAmountOfBoxes(Message) (Utilities|ResolveSoftReference (Variables|Default|GetWorkSticker)) (Utilities|Array|Length _outrownames))
      (for _index (range 0 (- (Utilities|Array|Length _outrownames) 1))
        (bind _returnvalue (Utilities|GetDataTableRow "/Game/Assets/DataTables/DT_BoxTypesForDay1.DT_BoxTypesForDay1" (Utilities|Array|Get(acopy) _outrownames _index))
          (:then
            (Utilities|Array|Add (Variables|Default|GetBoxesTypes) (.boxtype _returnvalue))))))
    (:1
      (bind _outrownames_2 (DataTable|GetDataTableRowNames "/Game/Assets/DataTables/DT_BoxTypesForDay2.DT_BoxTypesForDay2"))
      (Class|BPIAmountOfBoxes|SetAmountOfBoxes(Message) (Utilities|ResolveSoftReference (Variables|Default|GetWorkSticker)) (Utilities|Array|Length _outrownames_2))
      (for _index_2 (range 0 (- (Utilities|Array|Length _outrownames_2) 1))
        (bind _returnvalue_2 (Utilities|GetDataTableRow "/Game/Assets/DataTables/DT_BoxTypesForDay2.DT_BoxTypesForDay2" (Utilities|Array|Get(acopy) _outrownames_2 _index_2))
          (:then
            (Utilities|Array|Add (Variables|Default|GetBoxesTypes) (.boxtype _returnvalue_2))))))
    (:2
      (bind _outrownames_3 (DataTable|GetDataTableRowNames "/Game/Assets/DataTables/DT_BoxTypesForDay3.DT_BoxTypesForDay3"))
      (Class|BPIAmountOfBoxes|SetAmountOfBoxes(Message) (Utilities|ResolveSoftReference (Variables|Default|GetWorkSticker)) (Utilities|Array|Length _outrownames_3))
      (for _index_3 (range 0 (- (Utilities|Array|Length _outrownames_3) 1))
        (bind _returnvalue_3 (Utilities|GetDataTableRow "/Game/Assets/DataTables/DT_BoxTypesForDay3.DT_BoxTypesForDay3" (Utilities|Array|Get(acopy) _outrownames_3 _index_3))
          (:then
            (Utilities|Array|Add (Variables|Default|GetBoxesTypes) (.boxtype _returnvalue_3))))))))