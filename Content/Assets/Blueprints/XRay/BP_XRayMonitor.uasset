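; Clickable X-ray monitor actor whose screen the player switches on and off.
; Left-clicks require a valid, clickable item from BP_ItemSpawner and notify the player character, toggling the screen with on/off sounds only if it reports being in rotation.
; EnableMonitor makes the monitor box visible and collidable, and cursor hover highlights it through custom depth.
; A separate FlipFlop visibility function goes uncalled here, and IsInRotation always returns false.
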(event EventBeginPlay
  (bind _returnvalue (Actor|GetActorOfClass "/Game/Assets/Blueprints/Items/BP_ItemSpawner.BP_ItemSpawner_C"))
  (Variables|Default|SetItemSpawner _returnvalue))

(event EventEnableMonitor
  (Rendering|SetVisibility (Variables|Default|GetMonitors_Box001) true true)
  (Collision|SetCollisionEnabled (Variables|Default|GetMonitors_Box001) "QueryAndPhysics"))

(event MouseInput|EventActorBeginCursorOver
  (Rendering|SetRenderCustomDepth (Variables|Default|GetMonitors_Box001) true))

(event MouseInput|EventActorOnClicked
  (params (ButtonPressed :type Key%20Structure :default "None"))
  (bind _returnvalue (Game|GetPlayerCharacter 0))
  (bind _itemspawner (Variables|Default|GetItemSpawner))
  (bind _xrayscreen (Variables|Default|GetXRayScreen))
  (bind _itemonscene (Variables|/Game/Assets/Blueprints/Items/BP_ItemSpawner.BP_ItemSpawner_C|GetItemOnScene _itemspawner))
  (if (Utilities|IsValid _itemonscene)
    (if (and (== ButtonPressed "LeftMouseButton") (not (Variables|/Game/Assets/Blueprints/Items/BP_BaseItem.BP_BaseItem_C|GetnotClickable _itemonscene)))
      (Class|BPIXRay|ClickMonitor(Message) _returnvalue)
      (bind _inrotation (Class|BPIXRay|IsinRotation(Message) _returnvalue))
      (if _inrotation
        (if (Variables|Default|GetIsTurnOff)
          (Development|SetHiddeninGame _xrayscreen false false)
          (Variables|Default|SetIsTurnOff false)
          (Audio|Components|Audio|Play (Variables|Default|GetSC_TVTurnOn) 0.0)
          (else
            (Development|SetHiddeninGame _xrayscreen true false)
            (Variables|Default|SetIsTurnOff true)
            (Audio|Components|Audio|Play (Variables|Default|GetSC_TVTurnOff) 0.0)))))))

(event MouseInput|EventActorEndCursorOver
  (Rendering|SetRenderCustomDepth (Variables|Default|GetMonitors_Box001) false))

(fn ConstructionScript)

(fn ChangeScreenVisibility
  (bind _xrayscreen (Variables|Default|GetXRayScreen))
  (Utilities|FlowControl|FlipFlop
    (:A
      (Development|SetHiddeninGame _xrayscreen false false))
    (:B
      (Development|SetHiddeninGame _xrayscreen true false))))

(fn IsinRotation
  (return false))